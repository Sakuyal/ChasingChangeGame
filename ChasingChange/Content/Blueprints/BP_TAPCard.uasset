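; BP_TAPCard is a pickup actor that gives the BirdBoy character a temporary speed boost.
; When BirdBoy overlaps its box, it raises his MovementSpeed, hides itself, disables its collision and plays an explosion effect and sound.
; After a delay it sets MovementSpeed to a fixed lower value and destroys itself.
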(event OnComponentBeginOverlap(Box)
  (params (OverlappedComponent :type Primitive%20Component%20Object%20Reference) (OtherActor :type Actor%20Object%20Reference) (OtherComp :type Primitive%20Component%20Object%20Reference) (OtherBodyIndex :type Integer) (bFromSweep :type Boolean) (SweepResult :type Hit%20Result%20Structure%20%28by%20ref%29))
  (bind _returnvalue (Transformation|GetActorLocation))
  (bind _asbird_boy (Utilities|Casting|CastToBirdBoy OtherActor))
  (Variables|/Game/Blueprints/BirdBoy.BirdBoy_C|SetMovementSpeed _asbird_boy 1.5e+03)
  (Rendering|SetActorHiddenInGame true)
  (Collision|SetActorEnableCollision false)
  (Effects|SpawnEmitteratLocation "/Game/StarterContent/Particles/P_Explosion.P_Explosion" _returnvalue)
  (Audio|PlaySoundatLocation "/Game/StarterContent/Audio/Collapse02.Collapse02" _returnvalue "0, 0, 0" 1.0 1.0 0.0 0 0 0)
  (Utilities|FlowControl|Delay 15.0)
  (bind _asbird_boy_2 (Utilities|Casting|CastToBirdBoy OtherActor))
  (Variables|/Game/Blueprints/BirdBoy.BirdBoy_C|SetMovementSpeed _asbird_boy_2 7.5e+02)
  (Actor|DestroyActor))

(event EventBeginPlay)

(event Collision|EventActorBeginOverlap
  (params (OtherActor :type Actor%20Object%20Reference)))

(event EventTick
  (params (DeltaSeconds :type Float%20%28single-precision%29)))

(fn ConstructionScript)